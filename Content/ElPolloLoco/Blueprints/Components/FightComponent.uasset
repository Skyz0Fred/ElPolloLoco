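; FightComponent is an actor component that appears meant to drive attacks for its owning actor, though its logic is still a stub.
; On BeginPlay it stores the owner as Attacker and loops over the FightMoves array without acting on the entries.
; AttackButtonPressed and AttackInitiated lead into the same branch with a constant true condition and empty body.
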(event `self.ReceiveBeginPlay`
  (bind _fightmoves (`self.FightMoves`))
  (set `self.Attacker` (`self.GetOwner`))
  (if (> (`KismetArrayLibrary.Array_Length` _fightmoves) 0)
    (for _array_element _fightmoves
      _)))

(event `AttackInitiated`
  (if true :!label _label
    _))

(event `AttackButtonPressed`
  (goto _label))
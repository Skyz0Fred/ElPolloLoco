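; Health component that tracks an actor's health and signals when it dies.
; On BeginPlay it fills current health to the maximum and binds to the owner's OnTakeAnyDamage event.
; Each hit subtracts its damage and calls the OnDeath dispatcher whenever health is at or below zero, with no clamp or guard against repeat calls.
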(event `self.ReceiveBeginPlay`
  (set `self.CurrentHealth` (`self.MaxHealth`))
  (add `Actor.OnTakeAnyDamage` (`self.GetOwner`) (delegate `Event_TakeDamage`)))

(event `Event_TakeDamage`
  (params (DamagedActor :type "Actor Object Reference") (Damage :type "Float (double-precision)") (DamageType :type "DamageType Object Reference") (InstigatedBy :type "Controller Object Reference") (DamageCauser :type "Actor Object Reference"))
  (set `self.CurrentHealth` (- (`self.CurrentHealth`) Damage))
  (if (<= (`self.CurrentHealth`) 0.0)
    (`self.OnDeath`)))